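; BP_TextRenderer is an actor that displays world-space text that always faces the player's camera.
; Each Tick it rotates its TextRender component with a look-at rotation toward the first player's camera location, creating a billboard effect.
; SetTextInfo sets the text, world size and color, converting the linear color to an sRGB color.
; BeginPlay, overlap and construction logic are empty.
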(event EventBeginPlay)

(event Collision|EventActorBeginOverlap
  (params (OtherActor :type Actor%20Object%20Reference)))

(event EventTick
  (params (DeltaSeconds :type Float%20%28single-precision%29))
  (Transformation|SetWorldRotation (Variables|Default|GetTextRender) (Math|Rotator|FindLookatRotation (Transformation|GetWorldLocation (Variables|Default|GetTextRender)) (Camera|GetCameraLocation (Game|GetPlayerCameraManager 0))) false false))

(fn ConstructionScript)

(fn SetTextInfo
  (params (DisplayText :type Text) (DisplaySize :type Float%20%28double-precision%29) (DisplayColor :type Linear%20Color%20Structure))
  (Rendering|Components|TextRender|SetText (Variables|Default|GetTextRender) DisplayText)
  (Rendering|Components|TextRender|SetWorldSize (Variables|Default|GetTextRender) DisplaySize)
  (Rendering|Components|TextRender|SetTextRenderColor (Variables|Default|GetTextRender) (Math|Conversions|ToColor(LinearColor) DisplayColor)))