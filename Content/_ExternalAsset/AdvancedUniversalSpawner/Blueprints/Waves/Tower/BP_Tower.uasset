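; Defense tower that attacks non-player-controlled pawns entering a configurable box, sized and positioned in the construction script.
; On authority, overlaps maintain a target list, and a looping timer fires at a random target until none remain.
; By tower type, it applies delayed laser damage or spawns an aimed BP_LaserShot, adjusting the sphere material's rate.
; The brief laser beam effect spawns only in standalone or on remotes.
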(event OnComponentBeginOverlap(Box)
  (params (OverlappedComponent :type Primitive%20Component%20Object%20Reference) (OtherActor :type Actor%20Object%20Reference) (OtherComp :type Primitive%20Component%20Object%20Reference) (OtherBodyIndex :type Integer) (bFromSweep :type Boolean) (SweepResult :type Hit%20Result%20Structure%20%28by%20ref%29))
  (Networking|SwitchHasAuthority
    (:Authority
      (bind _as폰 (Utilities|Casting|CastToPawn OtherActor))
      (Utilities|IsValid _as폰
        (:Is%20Valid
          (if (not (Class|Controller|IsPlayerController (Pawn|GetController _as폰)))
            (Utilities|Array|Add (Variables|Default|GetTargets) _as폰)
            (if (not (Utilities|Time|IsTimerActivebyHandle (Variables|Default|GetTimer-Fire)))
              (bind _returnvalue (Utilities|Time|SetTimerbyFunctionName 0 "-Fire" (Variables|Default|GetAttackSpeed) true))
              (Variables|Default|SetTimer-Fire _returnvalue))))))))

(event OnComponentEndOverlap(Box)
  (params (OverlappedComponent :type Primitive%20Component%20Object%20Reference) (OtherActor :type Actor%20Object%20Reference) (OtherComp :type Primitive%20Component%20Object%20Reference) (OtherBodyIndex :type Integer))
  (Networking|SwitchHasAuthority
    (:Authority
      (bind _as폰 (Utilities|Casting|CastToPawn OtherActor))
      (Utilities|IsValid _as폰
        (:Is%20Valid
          (Utilities|Array|RemoveItem (Variables|Default|GetTargets) _as폰))))))

(event Custom|-BigLaser
  (params (Target :type Actor%20Object%20Reference))
  (CallFunction|-BigLaserMulti Target)
  (Utilities|FlowControl|Delay 0.25)
  (Utilities|IsValid Target
    (:Is%20Valid
      (Game|Damage|ApplyDamage Target (Variables|Default|GetDamage) 0 self))))

(event Custom|-BigLaserMulti
  (params (Param :type Actor%20Object%20Reference))
  (if (Class|KismetSystemLibrary|IsStandalone)
    _
    (else
      (Networking|SwitchHasAuthority
        (:Remote
          _))))
  (Utilities|IsValid Param
    (:Is%20Valid
      (bind _spawnedlaser (Variables|Default|GetSpawnedLaser)
        (:then
          (Components|DestroyComponent _spawnedlaser))
        (:else
          _))
      (bind _returnvalue (Effects|SpawnEmitterAttached "/Game/_ExternalAsset/AdvancedUniversalSpawner/DemoContent/Particles/P_Laser.P_Laser" (Variables|Default|GetSphere) "None"))
      (bind _output_get (Variables|Default|SetSpawnedLaser _returnvalue))
      (Effects|Components|ParticleSystem|SetActorParameter _output_get "Actor_Target" Param)
      (Utilities|FlowControl|Delay 0.25)
      (Components|DestroyComponent _output_get))))

(event EventBeginPlay
  (bind _sphere (Variables|Default|GetSphere))
  (bind _returnvalue (Rendering|Material|CreateDynamicMaterialInstance _sphere 0 (Rendering|Material|GetMaterial _sphere 0) "None" :!class /Script/Engine.PrimitiveComponent))
  (Variables|Default|SetDMI _returnvalue))

(fn ConstructionScript
  (bind _box (Variables|Default|GetBox))
  (Components|Box|SetBoxExtent _box (/ (Variables|Default|GetBoxExtent) (Transformation|GetActorScale3D)) true)
  (Transformation|SetRelativeLocation _box (Variables|Default|GetBoxExtent_Location) false false)
  (Rendering|SetVisibility _box (Variables|Default|GetVisibilityBoxExtent) false))

(fn -Fire
  (bind _sphere (Variables|Default|GetSphere))
  (bind _targets (Variables|Default|GetTargets))
  (bind _returnvalue (Transformation|GetWorldLocation _sphere))
  (Networking|SwitchHasAuthority
    (:Authority
      (if (> (Utilities|Array|Length (Variables|Default|GetTargets)) 0)
        (LocalVariables|Setlocal_Index (Math|Random|RandomIntegerinRange 0 (Utilities|Array|LastIndex _targets)))
        (Utilities|IsValid (Utilities|Array|Get(acopy) _targets (LocalVariables|Getlocal_Index))
          (:Is%20Valid
            (switch Utilities|FlowControl|Switch|SwitchonE_TowerType (Variables|Default|GetTowerType)
              (:NewEnumerator0
                (CallFunction|-BigLaser (Utilities|Array|Get(acopy) _targets (LocalVariables|Getlocal_Index)))
                (Rendering|Material|SetScalarParameterValue (Variables|Default|GetDMI) "Rate" 35.0 :!class /Script/Engine.MaterialInstanceDynamic))
              (:NewEnumerator1
                (Game|SpawnActorfromClass "/Game/_ExternalAsset/AdvancedUniversalSpawner/Blueprints/Waves/Tower/BP_LaserShot.BP_LaserShot_C" (Math|Transform|MakeTransform _returnvalue (Math|Rotator|FindLookatRotation _returnvalue (Transformation|GetActorLocation (Utilities|Array|Get(acopy) _targets (LocalVariables|Getlocal_Index)))) (* (Transformation|GetActorScale3D) 3.0)) "AlwaysSpawn" "OverrideRootScale" self (Variables|Default|GetDamage) 0)
                (Rendering|Material|SetScalarParameterValue (Variables|Default|GetDMI) "Rate" 2e+01 :!class /Script/Engine.MaterialInstanceDynamic))))
          (:Is%20Not%20Valid
            (Utilities|Array|RemoveIndex _targets (LocalVariables|Getlocal_Index))))
        (else
          (Utilities|Time|ClearandInvalidateTimerbyHandle (Variables|Default|GetTimer-Fire))
          (Rendering|Material|SetScalarParameterValue (Variables|Default|GetDMI) "Rate" 1e+01 :!class /Script/Engine.MaterialInstanceDynamic))))))