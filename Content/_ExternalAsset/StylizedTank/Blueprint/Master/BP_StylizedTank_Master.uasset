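; Master Blueprint for a player-driven tank with Enhanced Input driving, turning, camera aiming and projectile firing from every spawn-point component.
; Tick moves it kinematically, using BP_GroundSensing hit normals and heights to align body tilt and height to terrain.
; Turret yaw follows the camera, while gun pitch targets a camera line trace.
; Forward and turn speeds drive per-side track material scrolling and wheel animation values.
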(event Input|EnhancedActionEvents|EnhancedInputActionIA_Drive
  (params (ActionValue :type Float%20%28double-precision%29) (ElapsedSeconds :type Float%20%28double-precision%29) (TriggeredSeconds :type Float%20%28double-precision%29) (InputAction :type Input%20Action%20Object%20Reference :default "/Game/_ExternalAsset/StylizedTank/Inputs/IA_Drive.IA_Drive"))
  ;[1 1 1] Drive
  (:Triggered
    (Variables|Base|SetTargetForwardSpeed (* ActionValue (Variables|Base|GetMaxForwardSpeed))))
  (:Completed
    (Variables|Base|SetTargetForwardSpeed 0.0)))

(event Input|EnhancedActionEvents|EnhancedInputActionIA_Turn
  (params (ActionValue :type Float%20%28double-precision%29) (ElapsedSeconds :type Float%20%28double-precision%29) (TriggeredSeconds :type Float%20%28double-precision%29) (InputAction :type Input%20Action%20Object%20Reference :default "/Game/_ExternalAsset/StylizedTank/Inputs/IA_Turn.IA_Turn"))
  ;[1 1 1] Rotating Turret
  (:Triggered
    (Variables|Base|SetTargetTurnSpeed (* ActionValue (Variables|Base|GetMaxTurnSpeed))))
  (:Completed
    (Variables|Base|SetTargetTurnSpeed 0.0)))

(event Input|EnhancedActionEvents|EnhancedInputActionIA_Fire
  (params (ActionValue :type Boolean) (ElapsedSeconds :type Float%20%28double-precision%29) (TriggeredSeconds :type Float%20%28double-precision%29) (InputAction :type Input%20Action%20Object%20Reference :default "/Game/_ExternalAsset/StylizedTank/Inputs/IA_Fire.IA_Fire"))
  ;[1 1 1] Fire
  (for _array_element (Actor|GetComponentsByClass "/Game/_ExternalAsset/StylizedTank/Blueprint/Misc/Components/BP_ProjectileSpawnPoint.BP_ProjectileSpawnPoint_C")
    (Game|SpawnActorfromClass "/Game/_ExternalAsset/StylizedTank/Blueprint/Misc/Projectile/BP_Projectile_Master.BP_Projectile_Master_C" (Transformation|GetWorldTransform _array_element) "AdjustIfPossibleButAlwaysSpawn" "OverrideRootScale" 0 0)))

(event Input|EnhancedActionEvents|EnhancedInputActionIA_Turret
  (params (ActionValue :type Vector%202D%20Structure) (ElapsedSeconds :type Float%20%28double-precision%29) (TriggeredSeconds :type Float%20%28double-precision%29) (InputAction :type Input%20Action%20Object%20Reference :default "/Game/_ExternalAsset/StylizedTank/Inputs/IA_Turret.IA_Turret"))
  (bind (_x _y) (Math|Vector2D|BreakVector2D ActionValue))
  ;[1 1 1] Rotate View
  (Pawn|Input|AddControllerYawInput (* _x 0.25))
  (Pawn|Input|AddControllerPitchInput (* (* _y -1.0) 0.25)))

(event EventBeginPlay
  (bind _skeletalmesh (Variables|Default|GetSkeletalMesh))
  (bind _skeletalmesh_2 (Variables|Default|GetSkeletalMesh))
  (bind _returnvalue (Rendering|Material|GetMaterial _skeletalmesh_2 0))
  ;[1 1 1] Initialize
  (Utilities|FlowControl|Sequence
    (:then_0
      (Input|AddMappingContext (PlayerController|LocalPlayerSubsystems|GetEnhancedInputLocalPlayerSubsystem (Game|GetPlayerController 0)) "/Game/_ExternalAsset/StylizedTank/Inputs/IMC_Tank.IMC_Tank" 0 "(bIgnoreAllPressedKeysUntilRelease=True,bForceImmediately=False,bNotifyUserSettings=False)"))
    (:then_1
      ;[1 1 1] Get Ground Sensor Component
      (Variables|Base|SetGroundSensingArray (Actor|GetComponentsByClass "/Game/_ExternalAsset/StylizedTank/Blueprint/Misc/Components/BP_GroundSensing.BP_GroundSensing_C")))
    (:then_2
      ;[1 1 1] Obtain the track material to set up the UV animation
      (bind _returnvalue_2 (Rendering|Material|CreateDynamicMaterialInstance _skeletalmesh 0 _returnvalue "None" :!class /Script/Engine.PrimitiveComponent))
      (Variables|Base|SetRefLeftTrackMI _returnvalue_2)
      (bind _returnvalue_3 (Rendering|Material|CreateDynamicMaterialInstance _skeletalmesh 1 _returnvalue "None" :!class /Script/Engine.PrimitiveComponent))
      (Variables|Base|SetRefRightTrackMI _returnvalue_3))))

(event EventTick
  (params (DeltaSeconds :type Float%20%28single-precision%29))
  (bind _returnvalue (Utilities|Time|GetWorldDeltaSeconds))
  (bind _returnvalue_2 (Utilities|Time|GetWorldDeltaSeconds))
  (bind _targetturnspeed (Variables|Base|GetTargetTurnSpeed))
  (bind _returnvalue_3 (* _targetturnspeed 0.1))
  ;[1 1 1] Logic related to vehicle body ground alignment
  (Utilities|FlowControl|Sequence
    (:then_0
      (Variables|Base|SetTurretAngle (CallFunction|GetTurretAngle 1e+03))
      (Variables|Base|SetTurretGunAngle (CallFunction|GetGunAngle))
      (Variables|Base|SetAverageNormal "0, 0, 0")
      (Variables|Base|SetAverageHeight 0.0)
      (Variables|Base|SetCountOnGround 0))
    (:then_1
      (for _array_element (Variables|Base|GetGroundSensingArray)
        (Variables|Base|SetAverageNormal (+ (Variables|/Game/_ExternalAsset/StylizedTank/Blueprint/Misc/Components/BP_GroundSensing.BP_GroundSensing_C|GetHitNormal _array_element) (Variables|Base|GetAverageNormal)))
        (Variables|Base|SetAverageHeight (+ (.z (Variables|/Game/_ExternalAsset/StylizedTank/Blueprint/Misc/Components/BP_GroundSensing.BP_GroundSensing_C|GetHitLocation _array_element)) (Variables|Base|GetAverageHeight)))
        (if (Variables|/Game/_ExternalAsset/StylizedTank/Blueprint/Misc/Components/BP_GroundSensing.BP_GroundSensing_C|GetOnGround _array_element)
          (Math|Integer|IncrementInt (Variables|Base|GetCountOnGround))))
      (Variables|Base|SetAverageNormal (/ (Variables|Base|GetAverageNormal) (Variables|Base|GetCountOnGround)))
      (bind _output_get (Variables|Base|SetAverageHeight (/ (Variables|Base|GetAverageHeight) (Variables|Base|GetCountOnGround))))
      (Variables|Base|SetDeltaZ (- (+ _output_get (Variables|Base|GetHeightOffset)) (.z (Transformation|GetActorLocation))))
      (Transformation|SetActorRotation (Math|Interpolation|RInterpTo (Transformation|GetActorRotation) (Math|Rotator|CombineRotators (Math|Rotator|MakeRotator 0.0 0.0 (* (Variables|Base|GetTargetTurnSpeed) _returnvalue_2)) (Math|Rotator|MakeRotfromZY (Variables|Base|GetAverageNormal) (Transformation|GetActorRightVector))) _returnvalue_2 8.0))
      (Transformation|AddActorWorldOffset (+ (* (Transformation|GetActorForwardVector) (Math|Interpolation|FInterpTo (Variables|Base|GetCurrentForwardSpeed) (Variables|Base|GetTargetForwardSpeed) _returnvalue 1e+01) _returnvalue) (* (Transformation|GetActorUpVector) (Variables|Base|GetDeltaZ))) true true)
      (Variables|Base|SetCurrentForwardSpeed (Math|Interpolation|FInterpTo (Variables|Base|GetCurrentForwardSpeed) (Variables|Base|GetTargetForwardSpeed) _returnvalue 1e+01))
      ;[1 1 1] Set up track animation and wheel animation
      (Utilities|FlowControl|Sequence
        (:then_0
          (Rendering|Material|SetScalarParameterValue (Variables|Base|GetRefRightTrackMI) "TrackSpeed" (+ (* (Variables|Base|GetCurrentForwardSpeed) 0.005) _returnvalue_3) :!class /Script/Engine.MaterialInstanceDynamic)
          (if (> (+ (* (Variables|Base|GetCurrentForwardSpeed) 0.005) _returnvalue_3) 1.0)
            (bind _result (Math|Float|IncrementFloat (Variables|Base|GetWheel%20Speed%20R))
              (:%20%20
                (bind _output_get_2 (Variables|Base|SetWheel%20Speed%20R (* _result 1.0)))))
            (elif (== (+ (* (Variables|Base|GetCurrentForwardSpeed) 0.005) _returnvalue_3) 0.0)
              (Variables|Base|SetWheel%20Speed%20R _output_get_2)
              (else
                (bind _result_2 (Math|Float|DecrementFloat (Variables|Base|GetWheel%20Speed%20R))
                  (:%20%20
                    (Variables|Base|SetWheel%20Speed%20R (* _result_2 1.0))))))))
        (:then_1
          (Rendering|Material|SetScalarParameterValue (Variables|Base|GetRefLeftTrackMI) "TrackSpeed" (- (* (Variables|Base|GetCurrentForwardSpeed) 0.005) _returnvalue_3) :!class /Script/Engine.MaterialInstanceDynamic)
          (if (> (- (* (Variables|Base|GetCurrentForwardSpeed) 0.005) _returnvalue_3) 1.0)
            (bind _result_3 (Math|Float|IncrementFloat (Variables|Base|GetWheel%20Speed%20L))
              (:%20%20
                (bind _output_get_3 (Variables|Base|SetWheel%20Speed%20L (* _result_3 1.0)))))
            (elif (== (- (* (Variables|Base|GetCurrentForwardSpeed) 0.005) _returnvalue_3) 0.0)
              (Variables|Base|SetWheel%20Speed%20L _output_get_3)
              (else
                (bind _result_4 (Math|Float|DecrementFloat (Variables|Base|GetWheel%20Speed%20L))
                  (:%20%20
                    (Variables|Base|SetWheel%20Speed%20L (* _result_4 1.0))))))))))))

(fn ConstructionScript)

(fn GetTurretAngle
  (params (InSpeed :type Float%20%28double-precision%29))
  (bind _returnvalue (Class|KismetMathLibrary|VectorForward))
  (bind _camera (Variables|Default|GetCamera))
  (bind _returnvalue_2 (Math|Vector|GetForwardVector _camera))
  (bind _returnvalue_3 (Math|Vector|MakeVector (.x _returnvalue_2) (.y _returnvalue_2) 0.0))
  (bind _returnvalue_4 (Math|Vector|Normalize _returnvalue_3))
  (bind _returnvalue_5 (Math|Vector|DotProduct _returnvalue _returnvalue_4))
  (bind _returnvalue_6 (Class|KismetMathLibrary|DegAcos _returnvalue_5))
  (return (.Yaw (Math|Rotator|BreakRotator (Math|Interpolation|RInterpTo (Math|Rotator|MakeRotator 0.0 0.0 (Variables|Base|GetTurretAngle)) (Math|Rotator|MakeRotator 0.0 0.0 (- (Math|Float|SelectFloat _returnvalue_6 (- 3.6e+02 _returnvalue_6) (> (Math|Vector|DotProduct (Class|KismetMathLibrary|VectorRight) _returnvalue_4) 0.0)) (.yaw (Transformation|GetActorRotation)))) (Utilities|Time|GetWorldDeltaSeconds) InSpeed)))))

(fn GetGunAngle
  (bind _camera (Variables|Default|GetCamera))
  (bind _returnvalue (Transformation|GetWorldLocation _camera))
  (bind _returnvalue_2 (Math|Vector|GetForwardVector _camera))
  (bind _returnvalue_3 (* _returnvalue_2 7e+03))
  (bind _returnvalue_4 (+ _returnvalue _returnvalue_3))
  (Variables|Base|SetGunLocation _returnvalue_4)
  (bind (_outhit _returnvalue_5) (Collision|LineTraceForObjects _returnvalue _returnvalue_4 (Utilities|Array|MakeArray "ObjectTypeQuery1" "ObjectTypeQuery6" "ObjectTypeQuery2") false 0 "None"))
  (bind _output_get (Variables|Base|SetGunAngle (Math|Interpolation|FInterpTo (Variables|Base|GetGunAngle) (.pitch (Math|Rotator|FindLookatRotation (Transformation|GetSocketLocation (Variables|Default|GetSkeletalMesh) "Barrel") (select _returnvalue_5 (.Location (Collision|BreakHitResult _outhit)) (Variables|Base|GetGunLocation)))) (Utilities|Time|GetWorldDeltaSeconds) 5.0)))
  (return (* _output_get -1.0)))