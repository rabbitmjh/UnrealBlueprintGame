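; Jetpack backpack child actor that lets its parent Character hover on a limited pool of hover time.
; While activated, Tick drains HoverTime and calls LaunchCharacter with upward thrust, deactivating when time runs out.
; Activate and Deactivate swap the character's AirControl and toggle thrust VFX and sound; AddTime refills the pool.
; Every tick, a dynamic material's emissive color shows remaining time relative to InitHoverTime as a fuel gauge.
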(event Custom|ChangeBackpackColor
  (if (> (Variables|Default|GetHoverTime) (Variables|Default|GetInitHoverTime))
    (Rendering|Material|SetVectorParameterValue (Variables|Default|GetMID) "Emissive" "(R=10.000000,G=10.000000,B=10.000000,A=1.000000)" :!class /Script/Engine.MaterialInstanceDynamic)
    (elif (> (/ (Variables|Default|GetHoverTime) (Variables|Default|GetInitHoverTime)) 0.5)
      (Rendering|Material|SetVectorParameterValue (Variables|Default|GetMID) "Emissive" "(R=0.000000,G=10.000000,B=0.000000,A=1.000000)" :!class /Script/Engine.MaterialInstanceDynamic)
      (elif (> (/ (Variables|Default|GetHoverTime) (Variables|Default|GetInitHoverTime)) 0.3)
        (Rendering|Material|SetVectorParameterValue (Variables|Default|GetMID) "Emissive" "(R=10.000000,G=2.760965,B=0.000001,A=1.000000)" :!class /Script/Engine.MaterialInstanceDynamic)
        (elif (> (Variables|Default|GetHoverTime) 0.001)
          (Rendering|Material|SetVectorParameterValue (Variables|Default|GetMID) "Emissive" "(R=10.000000,G=0.000001,B=0.000000,A=1.000000)" :!class /Script/Engine.MaterialInstanceDynamic)
          (else
            (Rendering|Material|SetVectorParameterValue (Variables|Default|GetMID) "Emissive" "(R=0.000000,G=0.000000,B=0.000000,A=1.000000)" :!class /Script/Engine.MaterialInstanceDynamic)))))))

(event EventBeginPlay
  (bind _mesh (Variables|Default|GetMesh))
  (bind _as캐릭터 (Utilities|Casting|CastToCharacter (Actor|GetParentActor)))
  (Variables|Default|SetParentCharacter _as캐릭터)
  (bind _returnvalue (Rendering|Material|CreateDynamicMaterialInstance _mesh 0 (Rendering|Material|GetMaterial _mesh 0) "None" :!class /Script/Engine.PrimitiveComponent))
  (Variables|Default|SetMID _returnvalue))

(event Collision|EventActorBeginOverlap
  (params (OtherActor :type Actor%20Object%20Reference)))

(event EventTick
  (params (DeltaSeconds :type Float%20%28single-precision%29))
  (CallFunction|ChangeBackpackColor)
  (if (Variables|Default|GetbActivated)
    (bind _output_get (Variables|Default|SetHoverTime (- (Variables|Default|GetHoverTime) DeltaSeconds)))
    (if (> _output_get 0.0)
      (Character|LaunchCharacter (Variables|Default|GetParentCharacter) (Math|Vector|MakeVector 0.0 0.0 (Variables|Default|GetThrustPower)) false true)
      (else
        (CallFunction|DeactivateObject)))))

(event EventDeactivateObject
  (bind _thrustsfx (Variables|Default|GetThrustSFX))
  (bind _parentcharacter (Variables|Default|GetParentCharacter))
  (Utilities|IsValid _parentcharacter
    (:Is%20Valid
      (Variables|Default|SetbActivated false)
      (Variables|/Script/Engine.CharacterMovementComponent|SetAirControl (Variables|/Script/Engine.Character|GetCharacterMovement _parentcharacter) (Variables|Default|GetInitHoverSpeed))
      (Components|Activation|Deactivate (Variables|Default|GetThrustVFX))
      (if (Audio|Components|Audio|IsPlaying _thrustsfx)
        (Class|AudioParameterControllerInterface|SetTriggerParameter _thrustsfx "JetpackOff")))))

(event EventActivateObject
  (bind _parentcharacter (Variables|Default|GetParentCharacter))
  (Utilities|IsValid _parentcharacter
    (:Is%20Valid
      (Variables|Default|SetbActivated true)
      (Variables|/Script/Engine.CharacterMovementComponent|SetAirControl (Variables|/Script/Engine.Character|GetCharacterMovement _parentcharacter) (Variables|Default|GetHoverSpeed))
      (Components|Activation|Activate (Variables|Default|GetThrustVFX) false)
      (Audio|Components|Audio|Play (Variables|Default|GetThrustSFX) 0.0))))

(event EventAddTime
  (params (AddingTime :type Float%20%28double-precision%29))
  (Variables|Default|SetHoverTime (+ AddingTime (Variables|Default|GetHoverTime)))
  (Development|PrintString (Utilities|String|Append "남은 시간: " (Utilities|String|ToString(Float) (Variables|Default|GetHoverTime)))))

(fn ConstructionScript)

(fn GetHoverTime
  (return (Variables|Default|GetHoverTime)))