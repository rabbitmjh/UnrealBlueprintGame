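; Air strike actor that plays an incoming sound, waits out a warning time, then sets off a line of damaging explosions.
; A self-rescheduling timer steps from the actor's location along StrikeDirection by a fixed spacing, with random horizontal scatter.
; Each step spawns an effect, sound and falloff radial damage, each evaluating its own random offset, so their positions can differ.
; After the last explosion, the actor destroys itself following a short delay.
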(event Custom|StartBombing
  (Variables|Default|SetCurrentExplosionIndex 0)
  (CallFunction|SpawnNextExplosion))

(event Custom|SpawnNextExplosion
  (bind _returnvalue (Transformation|GetActorLocation))
  (bind _randomoffset (Variables|Default|GetRandomOffset))
  (bind _strikedirection (Variables|Default|GetStrikeDirection))
  (bind _explosionspacing (Variables|Default|GetExplosionSpacing))
  (bind _currentexplosionindex (Variables|Default|GetCurrentExplosionIndex))
  (bind _randomoffset_2 (Variables|Default|GetRandomOffset))
  (bind _randomoffset_3 (Variables|Default|GetRandomOffset))
  (bind _randomoffset_4 (Variables|Default|GetRandomOffset))
  (bind _returnvalue_2 (* _strikedirection _explosionspacing _currentexplosionindex))
  (bind _returnvalue_3 (* _randomoffset_2 -1.0))
  (bind _returnvalue_4 (* _randomoffset -1.0))
  (bind _returnvalue_5 (Math|Random|RandomFloatinRange _returnvalue_3 _randomoffset_3))
  (bind _returnvalue_6 (Math|Random|RandomFloatinRange _returnvalue_4 _randomoffset_4))
  (bind _returnvalue_7 (Math|Vector|MakeVector _returnvalue_6 _returnvalue_5 0.0))
  (bind _returnvalue_8 (+ _returnvalue _returnvalue_2 _returnvalue_7))
  (if (< (Variables|Default|GetCurrentExplosionIndex) (Variables|Default|GetExplosionCount))
    (Niagara|SpawnSystematLocation (Variables|Default|GetExplosionEffect) _returnvalue_8)
    (Audio|PlaySoundatLocation (Variables|Default|GetExplosionSound) _returnvalue_8 "0, 0, 0" 1.0 1.0 0.0 0 0 0 0)
    (Class|GameplayStatics|ApplyRadialDamagewithFalloff (Variables|Default|GetExplosionDamage) (Variables|Default|GetMinimumDamage) _returnvalue_8 (Variables|Default|GetInnerRadius) (Variables|Default|GetOuterRadius) 1.0 0 0 self (Game|GetInstigatorController) "ECC_Visibility")
    (Math|Integer|IncrementInt (Variables|Default|GetCurrentExplosionIndex)
      (:%20%20
        (Utilities|Time|SetTimerbyEvent (delegate Custom|SpawnNextExplosion) (Variables|Default|GetExplosionInterval))))
    (else
      (Utilities|FlowControl|Delay 2.0)
      (Actor|DestroyActor))))

(event EventBeginPlay
  (Audio|PlaySoundatLocation (Variables|Default|GetIncomingSound) (+ (Transformation|GetActorLocation) (* (Variables|Default|GetStrikeDirection) (Variables|Default|GetExplosionSpacing) (Variables|Default|GetCurrentExplosionIndex)) (Math|Vector|MakeVector (Math|Random|RandomFloatinRange (* (Variables|Default|GetRandomOffset) -1.0) (Variables|Default|GetRandomOffset)) (Math|Random|RandomFloatinRange (* (Variables|Default|GetRandomOffset) -1.0) (Variables|Default|GetRandomOffset)) 0.0)) "0, 0, 0" 1.0 1.0 0.0 0 0 0 0)
  (Utilities|Time|SetTimerbyEvent (delegate Custom|StartBombing) (Variables|Default|GetWarningTime)))

(event Collision|EventActorBeginOverlap
  (params (OtherActor :type Actor%20Object%20Reference)))

(event EventTick
  (params (DeltaSeconds :type Float%20%28single-precision%29)))

(fn ConstructionScript)