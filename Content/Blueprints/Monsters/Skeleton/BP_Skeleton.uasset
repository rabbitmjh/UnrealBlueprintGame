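; Skeleton monster Blueprint that adds visual and animation variety on top of its parent class.
; On BeginPlay it picks random left and right hand meshes and a random point light color, then makes both hand meshes follow the body mesh through leader pose.
; Attack, Die and TakeDamage ignore the incoming section name and pass a random numeric montage section name to the parent implementations.
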(event EventBeginPlay
  (|CallParentFunction)
  (Components|SkeletalMesh|SetSkeletalMeshAsset (Variables|Default|GetLeftHandMesh) (.OutItem (Utilities|Array|Random (Variables|Default|GetLeftHand))))
  (Components|SkeletalMesh|SetSkeletalMeshAsset (Variables|Default|GetRightHandMesh) (.OutItem (Utilities|Array|Random (Variables|Default|GetRightHand))))
  (Rendering|Components|Light|SetLightColor (Variables|Default|GetPointLight) (.OutItem (Utilities|Array|Random (Variables|Default|GetRandomLight))) true)
  (Components|SkinnedMesh|SetLeaderPoseComponent (Variables|Default|GetLeftHandMesh) (Variables|Character|GetMesh) false false))

(event Collision|EventActorBeginOverlap
  (params (OtherActor :type Actor%20Object%20Reference))
  (|CallParentFunction OtherActor) ; 지금 이 노드는 비활성 상태입니다. \n핀을 끌어서 다른 노드를 연결하면 활성화됩니다.
)

(event EventTick
  (params (DeltaSeconds :type Float%20%28single-precision%29))
  (|CallParentFunction DeltaSeconds) ; 지금 이 노드는 비활성 상태입니다. \n핀을 끌어서 다른 노드를 연결하면 활성화됩니다.
)

(fn ConstructionScript
  (|CallParentFunction))

(fn Attack
  (params (SectionName :type Name :default "None"))
  (|CallParentFunction (Utilities|String|StringToName (Utilities|String|ToString(Integer) (Math|Random|RandomIntegerinRange 0 (Variables|Default|GetMaxMontageAttackIndex))))))

(fn Die
  (params (SectionName :type Name :default "None"))
  (|CallParentFunction (Utilities|String|StringToName (Utilities|String|ToString(Integer) (Math|Random|RandomInteger (Variables|Default|GetMaxMontageDieIndex))))))

(fn TakeDamage
  (params (InDamage :type Float%20%28double-precision%29) (SectionName :type Name :default "None"))
  (|CallParentFunction InDamage (Utilities|String|StringToName (Utilities|String|ToString(Integer) (Math|Random|RandomInteger (Variables|Default|GetMaxMontageHitIndex))))))