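; Behavior tree decorator that passes when a monster's target is within its attack range.
; It requires a BP_MonsterBase pawn and a valid actor in the KeyTargetActor blackboard key.
; The distance is measured to the monster's own TargetActor, not the blackboard actor, and compared with the monster's AttackRange.
; The decorator's own AttackRange variable is unused.
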(fn PerformConditionCheckAI
  (params (OwnerController :type AI%20Controller%20Object%20Reference) (ControlledPawn :type Pawn%20Object%20Reference))
  (bind _asbp_monster_base (Utilities|Casting|CastToBP_MonsterBase ControlledPawn)
    (:then
      (Utilities|IsValid (AI|BehaviorTree|GetBlackboardValueasActor (Variables|Default|GetKeyTargetActor))
        (:Is%20Valid
          (if (>= (Variables|/Game/Blueprints/Monsters/BP_MonsterBase.BP_MonsterBase_C|GetAttackRange _asbp_monster_base) (Transformation|GetDistanceTo ControlledPawn (Variables|/Game/Blueprints/Monsters/BP_MonsterBase.BP_MonsterBase_C|GetTargetActor _asbp_monster_base)))
            (return true)
            (else
              _)))
        (:Is%20Not%20Valid
          _)))
    (:CastFailed
      _))
  (return false))