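; Dragonide lizard monster, a child Blueprint that adds armed and unarmed animation variants to its parent's combat behavior.
; On BeginPlay, HaveWeapon selects the attack montage and the section name used for hit and death reactions.
; Attack passes a random numbered section within that variant's max index to the parent.
; Attack, TakeDamage and Die ignore the incoming SectionName and substitute their own before calling the parent.
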(event EventBeginPlay
  (|CallParentFunction)
  (if (Variables|Default|GetbHaveWeapon)
    (Variables|Default|SetMontageSectionName (Variables|Default|GetNameWeapon))
    (Variables|Default|SetAttackMontage (Variables|Default|GetAttackWeapon))
    (else
      (Variables|Default|SetMontageSectionName (Variables|Default|GetNameUnarmed))
      (Variables|Default|SetAttackMontage (Variables|Default|GetAttackUnarmed)))))

(event Collision|EventActorBeginOverlap
  (params (OtherActor :type Actor%20Object%20Reference))
  (|CallParentFunction OtherActor) ; 지금 이 노드는 비활성 상태입니다. \n핀을 끌어서 다른 노드를 연결하면 활성화됩니다.
)

(event EventTick
  (params (DeltaSeconds :type Float%20%28single-precision%29))
  (|CallParentFunction DeltaSeconds) ; 지금 이 노드는 비활성 상태입니다. \n핀을 끌어서 다른 노드를 연결하면 활성화됩니다.
)

(fn ConstructionScript
  (|CallParentFunction))

(fn Attack
  (params (SectionName :type Name :default "None"))
  (if (Variables|Default|GetbHaveWeapon)
    (|CallParentFunction (Utilities|String|StringToName (Utilities|String|ToString(Integer) (Math|Random|RandomIntegerinRange 0 (Variables|Default|GetMaxMontageAttackWeaponIndex)))))
    (else
      (|CallParentFunction (Utilities|String|StringToName (Utilities|String|ToString(Integer) (Math|Random|RandomIntegerinRange 0 (Variables|Default|GetMaxMontageAttackUnarmedIndex))))))))

(fn TakeDamage
  (params (InDamage :type Float%20%28double-precision%29) (SectionName :type Name :default "None"))
  (|CallParentFunction InDamage (Variables|Default|GetMontageSectionName)))

(fn Die
  (params (SectionName :type Name :default "None"))
  (|CallParentFunction (Variables|Default|GetMontageSectionName)))