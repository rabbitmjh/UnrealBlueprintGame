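; Base monster character that targets the player and provides health, montage-based attacks, hit reactions and death, built for pooled reuse.
; EnableMonster resets state, collision and movement and runs the behavior tree, while DisableMonster hides it and calls an empty ReturnToPool.
; Attack stops AI movement and plays a named montage section.
; TakeDamage clamps HP, then plays a hit montage or calls Die, which stops AI logic, movement and collision.
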(event EventBeginPlay)

(event Collision|EventActorBeginOverlap
  (params (OtherActor :type Actor%20Object%20Reference)))

(event EventTick
  (params (DeltaSeconds :type Float%20%28single-precision%29)))

(fn ConstructionScript)

(fn InitializeMonster
  (Variables|Default|SetCurrentHP (Variables|Default|GetMaxHP))
  (Variables|Default|SetbIsDead false)
  (Variables|Default|SetbCanAttack true)
  (Rendering|SetActorHiddenInGame false)
  (Collision|SetActorEnableCollision true)
  (Actor|Tick|SetActorTickEnabled true)
  (Variables|/Script/Engine.CharacterMovementComponent|SetMaxWalkSpeed (Variables|Character|GetCharacterMovement) (Variables|Default|GetMoveSpeed))
  (Variables|Default|SetTargetActor (Game|GetPlayerCharacter 0)))

(fn Attack
  (params (Section%20Name :type Name))
  (if (Variables|Default|GetbIsDead)
    (return)
    (elif (Variables|Default|GetbCanAttack)
      (Utilities|IsValid (Variables|Default|GetTargetActor)
        (:Is%20Valid
          (Variables|Default|SetbCanAttack false)
          (AI|Navigation|StopMovement (AI|GetAIController self))
          (Animation|PlayAnimMontage (Variables|Montage|GetAttackMontage) 1.0 Section%20Name)
          (Utilities|Time|SetTimerbyEvent 0 (Variables|Default|GetAttackCooldown))
          (Variables|Default|SetbCanAttack true))
        (:Is%20Not%20Valid
          (return)))
      (else
        (return)))))

(fn Die
  (Variables|Default|SetbCanAttack false)
  (Variables|Default|SetbIsDead true)
  (AI|Logic|StopLogic (Variables|/Script/AIModule.AIController|GetBrainComponent (AI|GetAIController self)) "Die")
  (Pawn|Components|CharacterMovement|DisableMovement (Variables|Character|GetCharacterMovement))
  (Collision|SetActorEnableCollision false)
  (Animation|PlayAnimMontage (Variables|Montage|GetDeathMotage) 1.0 (Variables|Default|GetMontageSectionName)))

(fn DisableMonster
  (Rendering|SetActorHiddenInGame true)
  (Actor|Tick|SetActorTickEnabled false)
  (Variables|Default|SetTargetActor 0)
  (CallFunction|ReturntoPool))

(fn TakeDamage
  (params (InDamage :type Float%20%28double-precision%29))
  (if (Variables|Default|GetbIsDead)
    (return)
    (else
      (bind _output_get (Variables|Default|SetCurrentHP (Math|Float|Clamp(Float) (- (Variables|Default|GetCurrentHP) InDamage) 0.0 (Variables|Default|GetMaxHP))))
      (if (<= _output_get 0.0)
        (CallFunction|Die)
        (else
          (Animation|PlayAnimMontage (Variables|Montage|GetHitMontage) 1.0 (Variables|Default|GetMontageSectionName)))))))

(fn EnableMonster
  (Variables|Default|SetCurrentHP (Variables|Default|GetMaxHP))
  (Variables|Default|SetbIsDead false)
  (Variables|Default|SetbCanAttack true)
  (Rendering|SetActorHiddenInGame false)
  (Collision|SetCollisionEnabled (Variables|Collision|GetCapsuleComponent self) "QueryAndPhysics")
  (Collision|SetCollisionEnabled (Variables|Character|GetMesh) "QueryOnly")
  (Actor|Tick|SetActorTickEnabled true)
  (Pawn|Components|CharacterMovement|SetMovementMode (Variables|Character|GetCharacterMovement) "MOVE_Walking" 0)
  (Variables|Default|SetTargetActor (Game|GetPlayerCharacter 0))
  (bind _asai_컨트롤러 (Utilities|Casting|CastToAIController (Pawn|GetController)))
  (AI|RunBehaviorTree _asai_컨트롤러 (Variables|Default|GetBehaviorTree)))

(fn ReturntoPool)