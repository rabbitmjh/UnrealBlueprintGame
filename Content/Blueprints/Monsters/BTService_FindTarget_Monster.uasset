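; Behavior tree service that keeps a monster's combat target data current in the blackboard.
; Each tick it asks the controlled pawn for a target through FindTargetInterface, then writes the target actor and the distance to it.
; For pawns derived from BP_MonsterBase it also copies the attack range.
; When no valid target is returned, it clears only the target key, leaving distance and range untouched.
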(event EventReceiveTickAI
  (params (OwnerController :type AI%20Controller%20Object%20Reference) (ControlledPawn :type Pawn%20Object%20Reference) (DeltaSeconds :type Float%20%28single-precision%29))
  (if (Utilities|DoesObjectImplementInterface ControlledPawn (Variables|Default|GetFindTargetInterface))
    (bind _outtarget (Class|BPIFindTarget|FindTarget(Message) ControlledPawn))
    (Utilities|IsValid _outtarget
      (:Is%20Valid
        (Class|BTFunctionLibrary|SetBlackboardValueasObject (Variables|Default|GetKeyTargetActor) _outtarget)
        (Class|BTFunctionLibrary|SetBlackboardValueasFloat (Variables|Default|GetKeyDistance) (Transformation|GetDistanceTo ControlledPawn _outtarget))
        (bind _asbp_monster_base (Utilities|Casting|CastToBP_MonsterBase ControlledPawn))
        (Class|BTFunctionLibrary|SetBlackboardValueasFloat (Variables|Default|GetKeyAttackRange) (Variables|/Game/Blueprints/Monsters/BP_MonsterBase.BP_MonsterBase_C|GetAttackRange _asbp_monster_base)))
      (:Is%20Not%20Valid
        (Class|BTFunctionLibrary|SetBlackboardValueasObject (Variables|Default|GetKeyTargetActor))))))