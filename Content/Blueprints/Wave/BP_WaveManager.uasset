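; Wave manager that runs monster waves from per-wave Skeleton, Dragonide and armed Dragonide counts, updating the UI.
; On BeginPlay, if enabled, it caches the UI, monster pool and level spawn points, then starts wave one.
; Spawns use short timers, pulling pooled monsters near random spawn points via reachable-point sampling with capsule overlap checks.
; Death callbacks decrement the alive count, starting the next wave after a cooldown at zero.
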(event Custom|NextWave
  ;[1 1 1] 일정 시간 이후 다음 웨이브
  (Math|Integer|IncrementInt (Variables|Default|GetCurrentWave)
    (:%20%20
      (Utilities|FlowControl|Delay (Variables|Default|GetWaveCoolTime))
      (CallFunction|StartWave))))

(event Custom|SpawnOneMonster
  (bind _spawnpoints (Variables|Default|GetSpawnPoints))
  ;[1 1 1] 맵에 있는 스폰 포인트 중 랜덤으로 스폰
  (CallFunction|FindValidSpawnLocation (.location (Transformation|GetActorTransform (Utilities|Array|Get(acopy) _spawnpoints (Math|Random|RandomInteger (Utilities|Array|Length _spawnpoints))))))
  (bind _monster (Default|GetMonster (Variables|Default|GetPool) (Variables|Default|GetValidSpawnLocation%20) "0, 0, 0" (Variables|Default|GetNowSpawnMonster)))
  (EventDispatchers|UnbindallEventsfromOnMonsterDied _monster)
  (EventDispatchers|BindEventtoOnMonsterDied _monster (EventDispatchers|CreateEvent :!event Custom|OnMonsterDead))
  (Math|Integer|IncrementInt (Variables|Default|GetCurrentAliveMonster)
    (:%20%20
      (Math|Integer|IncrementInt (Variables|Default|GetSpawnedCount)))))

(event Custom|StartWave
  (bind _wbp_ui (Variables|Default|GetWBP%20UI))
  ;[1 1 1] 웨이브가 시작되면 UI에 전달, 지정된 마리 수만큼 소환
  (Variables|/Game/Blueprints/UI/WBP_UI.WBP_UI_C|SetWaveTextDelayTime _wbp_ui (Variables|Default|GetWaveCoolTime))
  (Variables|Default|SetSpawnSkeleton (.spawncount (.Skeleton (Utilities|Struct|BreakS_Monsters (Utilities|Array|Get(acopy) (Variables|Default|GetMonsterToSpawn) (- (Variables|Default|GetCurrentWave) 1))))))
  (Variables|Default|SetSpawnDragonide (.spawncount (.Dragonide (Utilities|Struct|BreakS_Monsters (Utilities|Array|Get(acopy) (Variables|Default|GetMonsterToSpawn) (- (Variables|Default|GetCurrentWave) 1))))))
  (Variables|Default|SetSpawnDragonide_Weapon (.spawncount (.Dragonide_Weapon (Utilities|Struct|BreakS_Monsters (Utilities|Array|Get(acopy) (Variables|Default|GetMonsterToSpawn) (- (Variables|Default|GetCurrentWave) 1))))))
  (Variables|/Game/Blueprints/UI/WBP_UI.WBP_UI_C|SetCurrentAlive _wbp_ui (+ (Variables|Default|GetSpawnSkeleton) (Variables|Default|GetSpawnDragonide) (Variables|Default|GetSpawnDragonide_Weapon)))
  (Variables|/Game/Blueprints/UI/WBP_UI.WBP_UI_C|SetCurrentWave _wbp_ui (Variables|Default|GetCurrentWave))
  (Default|SetWaveText _wbp_ui)
  (Variables|Default|SetCurrentAliveMonster 0)
  (Variables|Default|SetSpawnedCount 0)
  (for _index (range 1 (Variables|Default|GetSpawnSkeleton))
    (Variables|Default|SetNowSpawnMonster "/Game/Blueprints/Monsters/Skeleton/BP_Skeleton.BP_Skeleton_C")
    (Utilities|Time|SetTimerbyEvent (EventDispatchers|CreateEvent :!event Custom|SpawnOneMonster) 0.25))
  (for _index_2 (range 1 (Variables|Default|GetSpawnDragonide))
    (Variables|Default|SetNowSpawnMonster "/Game/Blueprints/Monsters/Lizard/Dragonide/BP_Dragonide.BP_Dragonide_C")
    (Utilities|Time|SetTimerbyEvent (EventDispatchers|CreateEvent :!event Custom|SpawnOneMonster) 0.25))
  (for _index_3 (range 1 (Variables|Default|GetSpawnDragonide_Weapon))
    (Variables|Default|SetNowSpawnMonster "/Game/Blueprints/Monsters/Lizard/Dragonide/BP_Dragonide_Weapon.BP_Dragonide_Weapon_C")
    (Utilities|Time|SetTimerbyEvent (EventDispatchers|CreateEvent :!event Custom|SpawnOneMonster) 0.25)))

(event Custom|OnMonsterDead
  (bind _currentalivemonster (Variables|Default|GetCurrentAliveMonster))
  ;[1 1 1] 몬스터가 다 죽으면 다음 웨이브
  (Math|Integer|DecrementInt _currentalivemonster
    (:%20%20
      (Variables|/Game/Blueprints/UI/WBP_UI.WBP_UI_C|SetCurrentAlive (Variables|Default|GetWBP%20UI) _currentalivemonster)
      (if (<= (Variables|Default|GetCurrentAliveMonster) 0)
        (CallFunction|NextWave)))))

(event EventBeginPlay
  ;[1 1 1] UI로 정보 전달, 맵에서 풀과 스폰포인트 저장 후 웨이브 시작
  (if (Variables|Default|GetbPlayWave)
    (Utilities|FlowControl|Delay 0.1)
    (bind _aspc_my_controller (Utilities|Casting|CastToPC_MyController (Game|GetPlayerController 0)))
    (Variables|Default|SetWBP%20UI (Variables|/Game/Framework/PC_MyController.PC_MyController_C|GetWBP%20UI _aspc_my_controller))
    (bind _returnvalue (Actor|GetActorOfClass "/Game/Blueprints/ObjectPool/BP_MonsterPool.BP_MonsterPool_C"))
    (Variables|Default|SetPool _returnvalue)
    (bind _outactors (Actor|GetAllActorsOfClass "/Game/Blueprints/Wave/BP_MonsterSpawnPoint.BP_MonsterSpawnPoint_C"))
    (Variables|Default|SetSpawnPoints _outactors)
    (Variables|Default|SetCurrentWave 1)
    (CallFunction|StartWave)))

(fn ConstructionScript)

(fn FindValidSpawnLocation
  (params (InOrigin :type Vector))
  (bind _randomradius (LocalVariables|GetRandomRadius))
  (bind _randomlocation (AI|Navigation|GetRandomReachablePointinRadius InOrigin _randomradius 0 0))
  (Utilities|FlowControl|ForLoopwithBreak 0 9 :!label _label
    (:LoopBody
      (bind _outactors (Collision|CapsuleOverlapActors _randomlocation (/ (LocalVariables|GetRandomRadius) 1e+01) 1.2e+02 (Utilities|Array|MakeArray "ObjectTypeQuery3") 0))
      (if (== (Utilities|Array|Length _outactors) 0)
        (Variables|Default|SetValidSpawnLocation%20 _randomlocation)
        (Variables|Default|SetbFoundLocation true)
        (goto _label Break)))))