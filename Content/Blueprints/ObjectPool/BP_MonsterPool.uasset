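; BP_MonsterPool is an object pool actor that supplies reusable monsters.
; On BeginPlay it spawns MonsterClass actors at the origin according to PoolSize, disables each, stores it in MonsterPool and prints its name.
; GetMonster enables the first hidden monster at the requested location and rotation and returns it, using the Hidden flag to mark availability.
; The pool does not grow when every monster is in use.
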(event EventBeginPlay
  (for _index (range 0 (Variables|Default|GetPoolSize))
    (bind _returnvalue (Game|SpawnActorfromClass (Variables|Default|GetMonsterClass) (Math|Transform|MakeTransform "0, 0, 0") "Undefined" "MultiplyWithRoot" 0 0))
    (Default|DisableMonster _returnvalue)
    (Utilities|Array|Add (Variables|Default|GetMonsterPool) _returnvalue)
    (Development|PrintString (Utilities|GetDisplayName _returnvalue))))

(event Collision|EventActorBeginOverlap
  (params (OtherActor :type Actor%20Object%20Reference)))

(event EventTick
  (params (DeltaSeconds :type Float%20%28single-precision%29)))

(fn ConstructionScript)

(fn GetMonster
  (params (SpawnLocation :type Vector) (SpawnRotation :type Rotator))
  (for _array_element (Variables|Default|GetMonsterPool)
    (if (Variables|/Script/Engine.Actor|GetbHidden _array_element)
      (Default|EnableMonster _array_element SpawnLocation SpawnRotation)
      (return _array_element))))