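; Base weapon Blueprint for a gun held by BP_Character, handling hitscan firing, ammo, reloading and recoil.
; SwitchTrigger feeds ShootBullet, which checks character state and ammo, re-arming a timer for automatic fire.
; Shooting traces randomized cones from the muzzle, using multiple traces for one weapon type, then applies point damage, doubled for headshots.
; Hits spawn decals, effects, physics force and monster-type-specific Niagara bursts; reload montages refill the clip on completion.
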(event Custom|ImpactFX
  (params (Emitter :type Particle%20System%20Object%20Reference) (AttachToComponent :type Scene%20Component%20Object%20Reference) (AttachPointName :type Name) (Location :type Vector) (DecalMaterial :type Material%20Interface%20Object%20Reference) (Rotation :type Rotator) (Target :type Primitive%20Component%20Object%20Reference))
  (bind _fp_gun (Variables|Default|GetFP_Gun))
  ;[1 1 1] 총알 발사
  ;;[0.4167 0.4167 0.4167] 임팩트 효과
  (Utilities|IsValid _fp_gun
    (:Is%20Valid
      (Effects|SpawnEmitterAttached "/Game/M4A1/Effects/MuzzleFlash/P_Muzzle.P_Muzzle" _fp_gun "Muzzle" (Transformation|GetSocketLocation _fp_gun "Muzzle") (Transformation|GetSocketRotation _fp_gun "Muzzle") "1.000000,1.000000,1.000000" "KeepWorldPosition")
      (Effects|SpawnEmitterAttached Emitter AttachToComponent AttachPointName Location Rotation "1.000000,1.000000,1.000000" "KeepWorldPosition")
      (Class|GameplayStatics|SpawnDecalAttached DecalMaterial "7.000000,7.000000,7.000000" AttachToComponent AttachPointName Location Rotation "KeepWorldPosition" 1.2e+02)
      (Audio|PlaySoundatLocation (Variables|Default|GetshootEffectSound) (Transformation|GetWorldLocation (Variables|Default|GetFP_Gun)) "0, 0, 0" 1.0 1.0 0.0 0 0 0 0)
      (Utilities|IsValid Target
        (:Is%20Valid
          (CallFunction|AddPhysics Target))))))

(event Custom|SetDamageShoot
  (params (HitResult :type Hit%20Result%20Structure))
  (bind (_bblockinghit _binitialoverlap _time _distance _location _impactpoint _normal _impactnormal _physmat _hitactor _hitcomponent _hitbonename) (Collision|BreakHitResult HitResult))
  ;[1 1 1] 총알 발사
  (bind _damage (CallFunction|Damage _hitbonename))
  (if (!= (Variables|Default|Getcharacter) _hitactor)
    (Game|Damage|ApplyPointDamage _hitactor _damage _location HitResult (Variables|Default|GettheInstigator) (Variables|Default|Getcharacter)))
  (CallFunction|ImpactFX "/Game/M4A1/Effects/MuzzleFlash/P_hit_effect.P_hit_effect" _hitcomponent _hitbonename _location "/Game/M4A1/Materials/MI_Bullet_Decals_Inst.MI_Bullet_Decals_Inst" (Math|Conversions|RotationFromXVector _normal) _hitcomponent))

(event Custom|reloading
  (bind _character (Variables|Default|Getcharacter))
  (bind _character_2 (Variables|Default|Getcharacter))
  (bind _clipsize (Variables|Default|GetClipSize))
  ;[1 1 1] 재장전
  (if (!= (Variables|Default|GetCurrentClip) _clipsize)
    (if (> (+ (Variables|Default|GetMaxClip) (Variables|Default|GetCurrentClip)) _clipsize)
      (Variables|Default|SetisReloading? true)
      (Animation|Montage|PlayMontage (Variables|Default|GetFP_Gun) (Variables|montage|GetReloadAnimMontage_Weapon) 1.2
        (:then
          (Variables|/Game/Blueprints/Player/BP_Character.BP_Character_C|SetisReloading _character true)
          (Animation|Montage|PlayMontage (Variables|/Script/Engine.Character|GetMesh _character) (Variables|montage|GetreloadAnimMontage) 1.2
            (:OnCompleted
              (Variables|/Game/Blueprints/Player/BP_Character.BP_Character_C|SetisReloading _character false)
              (Variables|Default|SetisReloading? false)
              (Variables|Default|SetMaxClip (+ (- (Variables|Default|GetCurrentClip) (Variables|Default|GetClipSize)) (Variables|Default|GetMaxClip)))
              (Variables|Default|SetCurrentClip (Variables|Default|GetClipSize))))))
      (elif (> (Variables|Default|GetMaxClip) 0)
        (Variables|Default|SetisReloading? true)
        (Animation|Montage|PlayMontage (Variables|Default|GetFP_Gun) (Variables|montage|GetReloadAnimMontage_Weapon) 1.2
          (:then
            (Variables|/Game/Blueprints/Player/BP_Character.BP_Character_C|SetisReloading _character_2 true)
            (Animation|Montage|PlayMontage (Variables|/Script/Engine.Character|GetMesh _character_2) (Variables|montage|GetreloadAnimMontage) 1.2
              (:OnCompleted
                (Variables|/Game/Blueprints/Player/BP_Character.BP_Character_C|SetisReloading _character_2 false)
                (Variables|Default|SetisReloading? false)
                (Variables|Default|SetCurrentClip (+ (Variables|Default|GetMaxClip) (Variables|Default|GetCurrentClip)))
                (Variables|Default|SetMaxClip 0)))))))))

(event Custom|recoil_event
  (bind _character (Variables|Default|Getcharacter))
  ;[1 1 1] 총알 발사
  (Utilities|IsValid _character
    (:Is%20Valid
      (Pawn|Input|AddControllerYawInput _character (Math|Random|RandomFloatinRange -1.0 1.0))
      (Pawn|Input|AddControllerPitchInput _character (Math|Random|RandomFloatinRange 0.2 -1.0))
      (if (Pawn|IsLocallyControlled _character)
        (Game|Feedback|ClientStartCameraShake (Game|GetPlayerController 0) "/Game/Blueprints/weapons/BP_ShootShake.BP_ShootShake_C" 1.0 "CameraLocal" "0, 0, 0")))))

(event Custom|MonsterHitNiagara
  (params (InHit :type Hit%20Result%20Structure))
  (bind (_bblockinghit _binitialoverlap _time _distance _location _impactpoint _normal _impactnormal _physmat _hitactor) (Collision|BreakHitResult InHit))
  (bind _returnvalue (Math|Rotator|MakeRotfromX _impactnormal))
  (bind _returnvalue_2 (* _impactnormal 2.0))
  (bind _returnvalue_3 (+ _impactpoint _returnvalue_2))
  ;[1 1 1] 총알 발사
  (bind _asbp_monster_base (Utilities|Casting|CastToBP_MonsterBase _hitactor))
  (switch Utilities|FlowControl|Switch|SwitchonE_MonsterType (Variables|/Game/Blueprints/Monsters/BP_MonsterBase.BP_MonsterBase_C|GetMonsterType _asbp_monster_base)
    (:NewEnumerator0
      (Niagara|SpawnSystematLocation "/Game/_ExternalAsset/Vefects/Blood_VFX/VFX/Performance_Versions/Bullet_Hits/One_Shot/OS_NS_Bullet_Hit_Small_White.OS_NS_Bullet_Hit_Small_White" _returnvalue_3 _returnvalue))
    (:NewEnumerator1
      (Niagara|SpawnSystematLocation "/Game/_ExternalAsset/Vefects/Blood_VFX/VFX/Performance_Versions/Bullet_Hits/One_Shot/OS_NS_Bullet_Hit_Large_Blue.OS_NS_Bullet_Hit_Large_Blue" _returnvalue_3 _returnvalue))))

(event Custom|playShootingMontage
  (bind _animweaponshootmontage (Variables|montage|GetAnimWeaponShootMontage))
  ;[1 1 1] 애니메이션 몽타주 재생
  (Animation|Montage|PlayMontage (Variables|/Script/Engine.Character|GetMesh (Variables|Default|Getcharacter)) (Variables|montage|GetanimShootingMontage)
    (:then
      (Utilities|IsValid _animweaponshootmontage
        (:Is%20Valid
          (Animation|Montage|PlayMontage (Variables|Default|GetFP_Gun) _animweaponshootmontage))))))

(event Custom|initializeWeapon
  ;[1 1 1] 무기 초기 세팅
  (Variables|Default|SetfieldOfView (Variables|/Script/Engine.CameraComponent|GetFieldOfView (Variables|Default|GetScopeCamera)))
  (Utilities|FlowControl|Delay 1e+01)
  (Physics|SetSimulatePhysics (Variables|Default|GetFP_Gun) false))

(event Custom|SwitchTrigger
  (params (isFiring :type Boolean) (Instigator :type Controller%20Object%20Reference) (Camera :type Camera%20Component%20Object%20Reference) (character :type Character%20Object%20Reference))
  ;[1 1 1] 총알 발사
  ;;[0.4375 0.4375 0.4375] 클라이언트에서의 명령
  (bind _asbp_character (Utilities|Casting|CastToBP_Character character))
  (Variables|Default|Setcharacter _asbp_character)
  (Variables|Default|SettheInstigator Instigator)
  (Variables|Default|SetcameraActive Camera)
  (Variables|Default|SetisFiring? isFiring)
  (CallFunction|ShootBullet))

(event Custom|addPhysics
  (params (AttachToComponent :type Primitive%20Component%20Object%20Reference))
  ;[1 1 1] 총알 발사
  ;;[0.4167 0.4167 0.4167] 임팩트 효과
  (if (Physics|IsSimulatingPhysics AttachToComponent "None")
    (Physics|AddForce AttachToComponent (* (Math|Vector|GetForwardVector (Variables|Default|GetcameraActive)) 5e+03) "None" true)))

(event Custom|Shooting
  (bind _cameraactive (Variables|Default|GetcameraActive))
  (bind _character (Variables|Default|Getcharacter))
  (bind _cameraactive_2 (Variables|Default|GetcameraActive))
  (bind _character_2 (Variables|Default|Getcharacter))
  ;[1 1 1] 총알 발사
  (if (Utilities|Enum|Equal(Enum) (Variables|Default|GetweaponType) "NewEnumerator2")
    (for _index (range 0 8)
      (bind _outhit (Collision|LineTraceByChannel (Transformation|GetSocketLocation (Variables|Default|GetFP_Gun) "Muzzle") (+ (Transformation|GetWorldLocation _cameraactive) (* (Class|KismetMathLibrary|RandomUnitVectorinEllipticalConeinDegrees (Math|Vector|GetForwardVector _cameraactive) (Variables|Default|GetSpread_Right) (Variables|Default|GetSpread_Up)) 1e+03)) "TraceTypeQuery2" false 0 "ForOneFrame"))
      (Utilities|IsValid _character
        (:Is%20Valid
          (Variables|/Game/Blueprints/Player/BP_Character.BP_Character_C|SetisShooting _character true)
          (CallFunction|SetDamageShoot _outhit)
          (CallFunction|MonsterHitNiagara _outhit))))
    (else
      (bind _outhit_2 (Collision|LineTraceByChannel (Transformation|GetSocketLocation (Variables|Default|GetFP_Gun) "Muzzle") (+ (Transformation|GetWorldLocation _cameraactive_2) (* (Class|KismetMathLibrary|RandomUnitVectorinEllipticalConeinDegrees (Math|Vector|GetForwardVector _cameraactive_2) (Variables|Default|GetSpread_Right) (Variables|Default|GetSpread_Up)) 1e+06)) "TraceTypeQuery2" false 0 "ForOneFrame"))
      (Utilities|IsValid _character_2
        (:Is%20Valid
          (Variables|/Game/Blueprints/Player/BP_Character.BP_Character_C|SetisShooting _character_2 true)
          (CallFunction|SetDamageShoot _outhit_2)
          (CallFunction|MonsterHitNiagara _outhit_2)))))
  (CallFunction|RecoilEvent))

(event EventBeginPlay
  ;[1 1 1] 무기 초기 세팅
  (CallFunction|InitializeWeapon))

(fn ConstructionScript)

(fn Damage
  (params (bone :type Name))
  (bind _damagemin (Variables|Default|GetDamageMin))
  ;[0.3 0.3 0.3] 헤드샷이면 대미지 2배
  (if (Utilities|Name|Equal(Name) bone "Head")
    (LocalVariables|SetdamageLocal (* _damagemin 2.0))
    (else
      (LocalVariables|SetdamageLocal _damagemin)))
  (return (LocalVariables|GetdamageLocal)))

(fn ShootBullet
  (bind _character (Variables|Default|Getcharacter))
  (bind _character_2 (Variables|Default|Getcharacter))
  (Utilities|IsValid _character
    (:Is%20Valid
      (if (Variables|/Game/Blueprints/Player/BP_Character.BP_Character_C|GetisHolstering? _character)
        (Variables|Default|SetisFiring? false :!label _label)
        (elif (Variables|/Game/Blueprints/Player/BP_Character.BP_Character_C|GetisReloading _character)
          (goto _label)
          (else
            _)))
      (if (Variables|Default|GetisFiring?)
        (if (> (Variables|Default|GetCurrentClip) 0)
          (Variables|Default|SetCurrentClip (- (Variables|Default|GetCurrentClip) 1))
          (switch Utilities|FlowControl|Switch|SwitchonFireModeEnum (Variables|Default|GetFiremode)
            (:NewEnumerator0
              (CallFunction|Shooting :!label _label_2))
            (:NewEnumerator1
              (goto _label_2))
            (:NewEnumerator2
              (CallFunction|Shooting)
              (Utilities|Time|SetTimerbyFunctionName 0 "shootBullet" (Variables|Default|GetshootSpeed))))
          (CallFunction|PlayShootingMontage)
          (else
            (Variables|Default|SetisFiring? false)
            (Utilities|IsValid _character_2 :!label _label_3
              (:Is%20Valid
                (Variables|/Game/Blueprints/Player/BP_Character.BP_Character_C|SetisShooting _character_2 false)))))
        (else
          (goto _label_3))))))