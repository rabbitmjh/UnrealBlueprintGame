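; BP_Grenade is a thrown grenade projectile that explodes when its fuse timer runs out.
; BeginPlay picks a random spin rate and starts the timer for Explode.
; Tick rotates the static mesh, scaling spin by ProjectileMovement speed so it slows as the grenade loses velocity.
; Explode runs once, spawning effect and sound, applying radial damage with falloff credited to the instigator, then destroying the actor.
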(event Custom|Explode
  (bind _returnvalue (Transformation|GetActorLocation))
  (if (not (Variables|Default|GetbExploded))
    (Variables|Default|SetbExploded true)
    (Niagara|SpawnSystematLocation (Variables|Default|GetExplosionEffect) _returnvalue)
    (Audio|PlaySoundatLocation (Variables|Default|GetExplosionSound) _returnvalue "0, 0, 0" 1.0 1.0 0.0 0 0 0 0)
    (Class|GameplayStatics|ApplyRadialDamagewithFalloff (Variables|Default|GetExplosionDamage) (Variables|Default|GetMinimumDamage) _returnvalue (Variables|Default|GetInnerRadius) (Variables|Default|GetOuterRadius) (Variables|Default|GetDamageFalloff) 0 0 self (Game|GetInstigatorController) "ECC_Visibility")
    (Actor|DestroyActor)))

(event EventBeginPlay
  (Variables|Default|SetGrenadeSpinSpeed (Math|Rotator|MakeRotator (Math|Random|RandomFloatinRange 4e+02 8e+02) (Math|Random|RandomFloatinRange -2e+02 2e+02) (Math|Random|RandomFloatinRange -5e+02 5e+02)))
  (Utilities|Time|SetTimerbyEvent (delegate Custom|Explode) (Variables|Default|GetFuseTime)))

(event Collision|EventActorBeginOverlap
  (params (OtherActor :type Actor%20Object%20Reference)))

(event EventTick
  (params (DeltaSeconds :type Float%20%28single-precision%29))
  ;[1 1 1] 수류탄이 일정 속도 내려가면 회전 멈춤
  (if true
    (Transformation|AddLocalRotation (Variables|Default|GetStaticMesh) (* (Variables|Default|GetGrenadeSpinSpeed) (* DeltaSeconds (Math|Float|MapRangeClamped (Math|Vector|VectorLength (Variables|/Script/Engine.MovementComponent|GetVelocity (Variables|Default|GetProjectileMovement))) 0.0 1.2e+03 0.0 1.0))) false false)))

(fn ConstructionScript)