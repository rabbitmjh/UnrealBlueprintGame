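; Behavior tree service that updates a drone AI's blackboard with its current target and combat state.
; Each tick it asks the controlled pawn for a target through FindTargetInterface, then writes the actor, a height-offset target location and the distance to it.
; It also copies range, attack, follow and has-target values from BP_Drone.
; When no valid target returns, it clears only the target actor key.
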(event EventReceiveTickAI
  (params (OwnerController :type AI%20Controller%20Object%20Reference) (ControlledPawn :type Pawn%20Object%20Reference) (DeltaSeconds :type Float%20%28single-precision%29))
  (if (Utilities|DoesObjectImplementInterface ControlledPawn (Variables|Default|GetFindTargetInterface))
    (bind _outtarget (Class|BPIFindTarget|FindTarget(Message) ControlledPawn))
    (Utilities|IsValid _outtarget
      (:Is%20Valid
        (Class|BTFunctionLibrary|SetBlackboardValueasObject (Variables|Default|GetKeyTargetActor) _outtarget)
        (bind _output_get (Variables|Default|SetCharacterLocation (Math|Vector|MakeVector (.x (Transformation|GetActorLocation _outtarget)) (.y (Transformation|GetActorLocation _outtarget)) (+ (.z (Transformation|GetActorLocation _outtarget)) (Variables|Default|GetZup)))))
        (AI|BehaviorTree|SetBlackboardValueasVector (Variables|Default|GetKeyTargetLocation) _output_get)
        (Class|BTFunctionLibrary|SetBlackboardValueasFloat (Variables|Default|GetKeyDistance) (Math|Vector|Distance(Vector) (Transformation|GetActorLocation ControlledPawn) (Variables|Default|GetCharacterLocation)))
        (bind _asbp_drone (Utilities|Casting|CastToBP_Drone ControlledPawn))
        (Class|BTFunctionLibrary|SetBlackboardValueasFloat (Variables|Default|GetKeyRange) (Variables|/Game/Blueprints/Drone/BP_Drone.BP_Drone_C|GetRange _asbp_drone))
        (Class|BTFunctionLibrary|SetBlackboardValueasBool (Variables|Default|GetKeyAttackMode) (Variables|/Game/Blueprints/Drone/BP_Drone.BP_Drone_C|GetbAttackMode _asbp_drone))
        (Class|BTFunctionLibrary|SetBlackboardValueasBool (Variables|Default|GetKeyFolowMode) (Variables|/Game/Blueprints/Drone/BP_Drone.BP_Drone_C|GetbFollowMode _asbp_drone))
        (Class|BTFunctionLibrary|SetBlackboardValueasBool (Variables|Default|GetKeyHasAttackTarget) (Variables|/Game/Blueprints/Drone/BP_Drone.BP_Drone_C|GetbHasAttackTarget _asbp_drone)))
      (:Is%20Not%20Valid
        (Class|BTFunctionLibrary|SetBlackboardValueasObject (Variables|Default|GetKeyTargetActor))))))